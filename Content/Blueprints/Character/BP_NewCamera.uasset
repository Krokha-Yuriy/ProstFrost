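; BP_NewCamera is a trigger-driven camera actor that becomes the view target when BP_Character enters its TriggerBox.
; On overlap, it stores itself in the character's NewCamera variable and calls SetViewTargetWithBlend on the first player controller.
; BeginPlay waits a zero-second delay, then applies the same switch if the player already overlaps the box.
; The construction script sets the box's transform and extent from variables.
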(event `self.ReceiveBeginPlay`
  (`KismetSystemLibrary.Delay` 0.0)
  (bind _asbp_character (cast `/Game/Blueprints/Character/BP_Character` (`GameplayStatics.GetPlayerPawn` 0)))
  (for _array_element (`self.GetOverlappingComponents` _asbp_character)
    (if (== _array_element (`self.TriggerBox`))
      (set `/Game/Blueprints/Character/BP_Character.NewCamera` self _asbp_character)
      (`PlayerController.SetViewTargetWithBlend` (`GameplayStatics.GetPlayerController` 0) self 0.0 "VTBlend_Linear" 0.0 false))))

(event `self.TriggerBox.OnComponentBeginOverlap`
  (params (OverlappedComponent :type "PrimitiveComponent Object Reference") (OtherActor :type "Actor Object Reference") (OtherComp :type "PrimitiveComponent Object Reference") (OtherBodyIndex :type Integer) (bFromSweep :type Boolean) (SweepResult :type "HitResult Structure (by ref)"))
  (bind _asbp_character (cast `/Game/Blueprints/Character/BP_Character` OtherActor))
  (set `/Game/Blueprints/Character/BP_Character.NewCamera` self _asbp_character)
  (`PlayerController.SetViewTargetWithBlend` (`GameplayStatics.GetPlayerController` 0) self 0.0 "VTBlend_Linear" 0.0 false))

(fn `UserConstructionScript`
  (`SceneComponent.K2_SetRelativeTransform` (`self.TriggerBox`) (`self.TriggerTransform`) false false)
  (`BoxComponent.SetBoxExtent` (`self.TriggerBox`) (`self.TriggerExtend`) true))