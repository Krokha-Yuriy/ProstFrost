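; BP_Shot is a projectile actor that deals damage to the first thing it hits and then removes itself.
; An overlap on its Box applies fixed damage to the other actor, with no filtering, and stops the ProjectileMovement.
; It sets both FBProjectile and FBHit visible, sets FBHit to non-looping playback, and destroys the actor after a short delay.
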(event `self.ReceiveBeginPlay`)

(event `self.Box.OnComponentBeginOverlap`
  (params (OverlappedComponent :type "PrimitiveComponent Object Reference") (OtherActor :type "Actor Object Reference") (OtherComp :type "PrimitiveComponent Object Reference") (OtherBodyIndex :type Integer) (bFromSweep :type Boolean) (SweepResult :type "HitResult Structure (by ref)"))
  (bind _fb_hit (`self.FB_Hit`))
  (`SceneComponent.SetVisibility` (`self.FB_Projectile`) true false)
  (`GameplayStatics.ApplyDamage` OtherActor 1.0)
  (`MovementComponent.StopMovementImmediately` (`self.ProjectileMovement`))
  (`SceneComponent.SetVisibility` _fb_hit true false)
  (`PaperFlipbookComponent.SetPlayRate` _fb_hit 1.0)
  (`PaperFlipbookComponent.SetLooping` _fb_hit false)
  (`KismetSystemLibrary.Delay` 0.1)
  (`self.K2_DestroyActor`))

(event `self.ReceiveTick`
  (params (DeltaSeconds :type "Float (single-precision)")))

(fn `UserConstructionScript`)