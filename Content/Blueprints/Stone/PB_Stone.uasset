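; Pushable stone block that the player character shoves a set travel distance along a forward vector.
; Push runs CanPuch, which uses line and box traces to reject blocked paths, missing floor, blocks on top or a jumping player.
; A valid push disables player movement, attaches the player to the block and moves it with the MoveBlock timeline, then StopPushing restores walking and detaches.
; The path and floor trace offsets keep only the X component.
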(event `Push`
  (bind _returnvalue (`GameplayStatics.GetPlayerCharacter` 0))
  ;[1 1 1] Push
  (set `self.CurrentLocation` (`self.K2_GetActorLocation`))
  (set `self.PushableDirection` (`self.GetActorForwardVector` (stale `self.ReceiveHit` Other)))
  (bind _canpush (`self.CanPuch`))
  (if _canpush
    (`CharacterMovementComponent.DisableMovement` (`Character.CharacterMovement` _returnvalue))
    (`self.K2_AttachToActor` _returnvalue self "None" "KeepWorld" "KeepWorld" "KeepWorld" true)
    (bind (_direction _position) (`Timeline|MoveBlock` :!via `PlayFromStart`)
      (:`Update`
        (`self.K2_SetActorRelativeLocation` (+ (* _position (`self.PushableDirection`) (`self.TravelDistance`)) (`self.CurrentLocation`))))
      (:`Finished`
        (`self.StopPushing`)))))

(event `self.ReceiveHit`
  (params (MyComp :type "PrimitiveComponent Object Reference") (Other :type "Actor Object Reference") (OtherComp :type "PrimitiveComponent Object Reference") (bSelfMoved :type Boolean) (HitLocation :type "Vector Structure") (HitNormal :type "Vector Structure") (NormalImpulse :type "Vector Structure") (Hit :type "HitResult Structure (by ref)"))
  ;[1 1 1] Push
)

(event `StopPushing`
  (bind _returnvalue (`GameplayStatics.GetPlayerCharacter` 0))
  ;[1 1 1] Stop pushing
  (`CharacterMovementComponent.SetMovementMode` (`Character.CharacterMovement` _returnvalue) "MOVE_Walking" 0)
  (`self.K2_DetachFromActor` _returnvalue "KeepWorld" "KeepWorld" "KeepWorld"))

(event `/Game/Interfeises/BPI_CharacterMovement.CharacterMovement`
  (params (MovementScale :type "Float (double-precision)")))

(event `/Game/Interfeises/BPI_CharacterMovement.CharacterJump`
  (params (InJump :type Boolean))
  (set `self.InJump` InJump))

(fn `CanPuch`
  (returns (CanPush :type Boolean))
  (locals (CanPuchLocal :type Boolean :default true))
  (bind _returnvalue (`self.K2_GetActorLocation`))
  (bind _returnvalue_2 (`self.K2_GetActorLocation`))
  (bind _returnvalue_3 (`GameplayStatics.GetPlayerCharacter` 0))
  (bind _stoneblock (`self.StoneBlock`))
  (bind _returnvalue_4 (`self.K2_GetActorLocation` _returnvalue_3))
  (bind (_relativescale3d_x _relativescale3d_y _relativescale3d_z) (`KismetMathLibrary.BreakVector` (`SceneComponent.RelativeScale3D` _stoneblock)))
  (bind _returnvalue_5 (`StaticMesh.GetBounds` (`StaticMeshComponent.StaticMesh` _stoneblock)))
  (bind _returnvalue_6 (+ (`self.K2_GetActorLocation`) (* (`self.PushableDirection`) (`self.TravelDistance`) (3.0 0.0 0.0) 1.5)))
  (`|ExecutionSequence`
    (:`then_0`
      ;[1 1 1 1 50] Is there a block in front of character
      (bind (_outhit _returnvalue_7) (`KismetSystemLibrary.LineTraceSingle` _returnvalue_4 (+ _returnvalue_4 (* (`self.GetActorForwardVector` _returnvalue_3) 100.0)) "TraceTypeQuery1" false (`|MakeArray` _returnvalue_3) "None" false))
      (if _returnvalue_7
        (if (not (== (`.HitActor` (`GameplayStatics.BreakHitResult` _outhit)) self))
          (set `local.CanPuchLocal` false))))
    (:`then_1`
      ;[1 0.01891 0 1 50] Is there a block interference behind block
      (bind (_outhit_2 _returnvalue_8) (`KismetSystemLibrary.BoxTraceSingle` _returnvalue_2 (+ _returnvalue_2 (* (`self.PushableDirection`) (`self.TravelDistance`) (1.5 0.0 0.0))) (* (`KismetMathLibrary.MakeVector` (.x (`.BoxExtent` (`KismetMathLibrary.BreakBoxSphereBounds` _returnvalue_5))) 0.0 (.z (`.BoxExtent` (`KismetMathLibrary.BreakBoxSphereBounds` _returnvalue_5)))) (`KismetMathLibrary.MakeVector` _relativescale3d_x 0.0 _relativescale3d_z) (3.0 0.0 3.0)) (struct) "TraceTypeQuery1"))
      (if (not (not _returnvalue_8))
        (set `local.CanPuchLocal` false)))
    (:`then_2`
      ;[1 1 1 1 50] There is a floor under block
      (bind (_outhit_3 _returnvalue_9) (`KismetSystemLibrary.LineTraceSingle` _returnvalue_6 (+ _returnvalue_6 (0.0 0.0 -200.0)) "TraceTypeQuery1"))
      (if (not _returnvalue_9)
        (set `local.CanPuchLocal` false)))
    (:`then_3`
      ;[1 1 1 1 50] Is there a block above block
      (bind (_outhit_4 _returnvalue_10) (`KismetSystemLibrary.LineTraceSingle` _returnvalue (+ _returnvalue (0.0 0.0 200.0)) "TraceTypeQuery1"))
      (if _returnvalue_10
        (set `local.CanPuchLocal` false)))
    (:`then_4`
      ;[1 1 1 1 50] A character in a jump
      (if (`self.InJump`)
        (set `local.CanPuchLocal` false)))
    (:`then_5`
      (return (`local.CanPuchLocal`)))))

(fn `UserConstructionScript`)